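; BP_Sphere is a physics sphere that splits into smaller generations of itself with Niagara bursts until it vanishes.
; StartSplitS spawns copies at six child scene points, passing on the generation, until a per-instance random limit is exceeded.
; Non-first spheres launch in random directions with a brief emissive flash, with hue offset by generation through a dynamic material.
; Vanishing enlarges SearchVolume to knock and flash overlapping spheres before destroying itself.
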(event `self.ReceiveBeginPlay`
  (bind _spawnlocations (`self.SpawnLocations`))
  (bind _midsphere (`self.MidSphere`))
  (`KismetArrayLibrary.Array_Add` _spawnlocations (`self.P1`))
  (`KismetArrayLibrary.Array_Add` _spawnlocations (`self.P2`))
  (`KismetArrayLibrary.Array_Add` _spawnlocations (`self.P3`))
  (`KismetArrayLibrary.Array_Add` _spawnlocations (`self.P4`))
  (`KismetArrayLibrary.Array_Add` _spawnlocations (`self.P6`))
  (`KismetArrayLibrary.Array_Add` _spawnlocations (`self.P5`))
  (bind _returnvalue (`PrimitiveComponent.CreateDynamicMaterialInstance` (`self.Sphere`) 0 "/Game/_MAT/MI_cube.MI_cube" "None"))
  (bind _output_get (set `self.MidSphere` _returnvalue))
  (`MaterialInstanceDynamic.SetScalarParameterValue` _output_get "HueOffset" (`KismetMathLibrary.Conv_IntToDouble` (`self.GenerationS`)))
  (set `self.MaxGenerationsS` (`KismetMathLibrary.RandomIntegerInRange` 1 4))
  (if (not (`self.FirstSphere?`))
    (`PrimitiveComponent.AddImpulse` (`self.Sphere`) (* (`KismetMathLibrary.RandomUnitVector`) (`self.ImpluseScalarS`)) "None" true)
    (`MaterialInstanceDynamic.SetScalarParameterValue` _midsphere "Emission" 5.0)
    (`KismetSystemLibrary.Delay` 0.1)
    (`MaterialInstanceDynamic.SetScalarParameterValue` _midsphere "Emission" 0.0)))

(event `StartSplitS`
  (bind _result (`/Engine/EditorBlueprintResources/StandardMacros.IncrementInt` (`self.GenerationS`))
    (:`  `
      (if (<= _result (`self.MaxGenerationsS`))
        (`self.DisableParentSphere`)
        (`self.SpawnSpheres`)
        (else
          (`self.Vanish`))))))

(event `SpawnSpheres`
  (bind (_returnvalue_location _returnvalue_rotation _returnvalue_scale) (`KismetMathLibrary.BreakTransform` (`self.GetTransform`)))
  (`NiagaraFunctionLibrary.SpawnSystemAtLocation` "/Game/_FX/NS_Burst.NS_Burst" _returnvalue_location _returnvalue_rotation _returnvalue_scale)
  (for _array_element (`self.SpawnLocations`)
    (`|SpawnActorFromClass` "BP_Sphere_C" (`KismetMathLibrary.MakeTransform` (`SceneComponent.K2_GetComponentLocation` _array_element) (`SceneComponent.K2_GetComponentRotation` _array_element) (* (`SceneComponent.RelativeScale3D` _array_element) (`self.GetActorScale3D`))) "Undefined" "MultiplyWithRoot" null (`self.GenerationS`) null))
  (`self.K2_DestroyActor`))

(event `Vanish`
  (bind (_returnvalue_location _returnvalue_rotation _returnvalue_scale) (`KismetMathLibrary.BreakTransform` (`self.GetTransform`)))
  (`SceneComponent.SetRelativeScale3D` (`self.SearchVolume`) (4.0 4.0 4.0))
  (for _array_element (`PrimitiveComponent.GetOverlappingActors` (`self.SearchVolume`) "BP_Sphere_C")
    (bind _asbp_sphere (cast `/Game/_BP/BP_Sphere` _array_element))
    (`self.Searched` _asbp_sphere))
  (`NiagaraFunctionLibrary.SpawnSystemAtLocation` "/Game/_FX/NS_Burst.NS_Burst" _returnvalue_location (struct) _returnvalue_scale)
  (`self.DisableParentSphere`)
  (`self.K2_DestroyActor`))

(event `Searched`
  (bind (_returnvalue_location _returnvalue_rotation _returnvalue_scale) (`KismetMathLibrary.BreakTransform` (`self.GetTransform`)))
  (`NiagaraFunctionLibrary.SpawnSystemAtLocation` "/Game/_FX/NS_Burst.NS_Burst" _returnvalue_location _returnvalue_rotation _returnvalue_scale)
  (`PrimitiveComponent.AddImpulse` (`self.Sphere`) (* (`KismetMathLibrary.RandomUnitVector`) 400.0) "None" true)
  (bind _returnvalue (`PrimitiveComponent.CreateDynamicMaterialInstance` (`self.Sphere`) 0 "/Game/_MAT/MI_cube.MI_cube" "None"))
  (bind _output_get (set `self.MidSphere` _returnvalue))
  (`MaterialInstanceDynamic.SetScalarParameterValue` _output_get "HueOffset" (`KismetMathLibrary.Conv_IntToDouble` (`self.GenerationS`)))
  (`MaterialInstanceDynamic.SetScalarParameterValue` _output_get "Emission" 5.0)
  (`KismetSystemLibrary.Delay` 0.1)
  (`MaterialInstanceDynamic.SetScalarParameterValue` _output_get "Emission" 0.0))

(fn `DisableParentSphere`
  (bind _sphere (`self.Sphere`))
  (`PrimitiveComponent.SetSimulatePhysics` _sphere false)
  (`PrimitiveComponent.SetCollisionEnabled` _sphere "NoCollision")
  (`PrimitiveComponent.SetCollisionObjectType` _sphere "ECC_WorldStatic"))

(fn `UserConstructionScript`)